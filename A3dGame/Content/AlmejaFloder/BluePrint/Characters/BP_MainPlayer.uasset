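; Player character Blueprint with Enhanced Input movement, look, jump and crouch, plus shooting and weapon switching.
; Shooting line-traces from ShootPoint and applies fixed damage to hit Characters, with the trace end multiplying start location by scaled camera forward rather than adding it.
; The mouse wheel cycles a wrapping index over three blade meshes (baguette, balloon, fish).
; GetWeapon hides all meshes, then shows and attaches the current one to the right-hand socket.
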(event Input|EnhancedActionEvents|EnhancedInputActionIA_Crouch
  (params (ActionValue :type Boolean) (ElapsedSeconds :type Float%20%28double-precision%29) (TriggeredSeconds :type Float%20%28double-precision%29) (InputAction :type Input%20Action%20Object%20Reference :default "/Game/AlmejaFloder/Inputs/IA_Crouch.IA_Crouch"))
  (:Started
    (Character|Crouch))
  (:Canceled
    (Character|UnCrouch :!label _label))
  (:Completed
    (goto _label)))

(event Input|EnhancedActionEvents|EnhancedInputActionIA_CustomMove
  (params (ActionValue :type Vector%202D%20Structure) (ElapsedSeconds :type Float%20%28double-precision%29) (TriggeredSeconds :type Float%20%28double-precision%29) (InputAction :type Input%20Action%20Object%20Reference :default "/Game/AlmejaFloder/Inputs/IA_CustomMove.IA_CustomMove"))
  (bind _returnvalue (Pawn|GetControlRotation :!class /Script/Engine.Pawn))
  (Class|PawnMovementComponent|AddInputVector (Variables|Character|GetCharacterMovement) (* (.x ActionValue) (Math|Vector|GetRightVector (Math|Rotator|MakeRotator (.roll _returnvalue) 0.0 (.yaw _returnvalue)))) false)
  (Class|PawnMovementComponent|AddInputVector (Variables|Character|GetCharacterMovement) (* (.y ActionValue) (Math|Vector|GetForwardVector (Math|Rotator|MakeRotator 0.0 0.0 (.yaw (Pawn|GetControlRotation :!class /Script/Engine.Pawn))))) false))

(event Input|EnhancedActionEvents|EnhancedInputActionIA_CustomLoock
  (params (ActionValue :type Vector%202D%20Structure) (ElapsedSeconds :type Float%20%28double-precision%29) (TriggeredSeconds :type Float%20%28double-precision%29) (InputAction :type Input%20Action%20Object%20Reference :default "/Game/AlmejaFloder/Inputs/IA_CustomLoock.IA_CustomLoock"))
  (Pawn|Input|AddControllerYawInput (.x ActionValue))
  (Pawn|Input|AddControllerPitchInput (.y ActionValue)))

(event Input|EnhancedActionEvents|EnhancedInputActionIA_CustomJump
  (params (ActionValue :type Boolean) (ElapsedSeconds :type Float%20%28double-precision%29) (TriggeredSeconds :type Float%20%28double-precision%29) (InputAction :type Input%20Action%20Object%20Reference :default "/Game/AlmejaFloder/Inputs/IA_CustomJump.IA_CustomJump"))
  (:Started
    (Character|Jump)))

(event Input|EnhancedActionEvents|EnhancedInputActionIA_CustomShoot
  (params (ActionValue :type Boolean) (ElapsedSeconds :type Float%20%28double-precision%29) (TriggeredSeconds :type Float%20%28double-precision%29) (InputAction :type Input%20Action%20Object%20Reference :default "/Game/AlmejaFloder/Inputs/IA_CustomShoot.IA_CustomShoot"))
  (bind _distance (Variables|Default|GetDistance))
  (bind _shootpoint (Variables|Default|GetShootPoint))
  (bind _returnvalue (Transformation|GetWorldLocation _shootpoint))
  (:Started
    (bind _outhit (Collision|LineTraceByChannel _returnvalue (* _returnvalue (* (Math|Vector|GetForwardVector (Variables|Default|GetCamera)) (Math|Vector|MakeVector _distance _distance 0.0))) "TraceTypeQuery2" false 0 "ForDuration"))
    (bind _ascharacter (Utilities|Casting|CastToCharacter (.HitActor (Collision|BreakHitResult _outhit))))
    (Game|Damage|ApplyDamage _ascharacter 5.0 0 0)))

(event EventBeginPlay
  (bind _asplayer_controller (Utilities|Casting|CastToPlayerController (Pawn|GetController)))
  (Input|AddMappingContext (PlayerController|LocalPlayerSubsystems|GetEnhancedInputLocalPlayerSubsystem _asplayer_controller) "/Game/AlmejaFloder/Inputs/BP_GameRemake.BP_GameRemake" 0 "(bIgnoreAllPressedKeysUntilRelease=True,bForceImmediately=False,bNotifyUserSettings=False)")
  (bind _output_get (Variables|Default|SetWeaponInventory (Utilities|Array|MakeArray (Variables|Default|GetSK_Blade_Baguette) (Variables|Default|GetSK_Blade_Balloon) (Variables|Default|GetSK_Blade_Fish))))
  (CallFunction|GetWeapon _output_get))

(event Collision|EventActorBeginOverlap
  (params (OtherActor :type Actor%20Object%20Reference)))

(event EventTick
  (params (DeltaSeconds :type Float%20%28single-precision%29)))

(event Input|MouseEvents|MouseWheelAxis
  (params (AxisValue :type Float%20%28single-precision%29))
  (if (Utilities|Array|IsValidIndex (Variables|Default|GetWeaponInventory) (Math|Float|Truncate (+ AxisValue (Variables|Default|GetCurrentWeapon))))
    (Variables|Default|SetCurrentWeapon (Math|Float|Truncate (+ AxisValue (Variables|Default|GetCurrentWeapon))))
    (CallFunction|GetWeapon (Variables|Default|GetWeaponInventory))
    (elif (< (Math|Float|Truncate (+ AxisValue (Variables|Default|GetCurrentWeapon))) 0)
      (Variables|Default|SetCurrentWeapon (Utilities|Array|LastIndex (Variables|Default|GetWeaponInventory)))
      (CallFunction|GetWeapon (Variables|Default|GetWeaponInventory))
      (else
        (Variables|Default|SetCurrentWeapon 0)
        (CallFunction|GetWeapon (Variables|Default|GetWeaponInventory))))))

(fn ConstructionScript)

(fn GetWeapon
  (params (Array :type Array%20of%20Skeletal%20Mesh%20Component%20Object%20References))
  (bind _currentweapon (Variables|Default|GetCurrentWeapon))
  (bind _output (Utilities|Array|Get(acopy) Array _currentweapon))
  (for _array_element Array
    (Rendering|SetVisibility _array_element false false))
  (Rendering|SetVisibility _output true false)
  (Transformation|AttachComponentToComponent _output (Variables|Character|GetMesh) "Weapoin_RightHand_Socket" "SnapToTarget" "KeepRelative" "KeepRelative" true))