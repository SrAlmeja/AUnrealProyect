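; BP_NPC is a character that follows the player and turns into a ragdoll when damaged.
; Every Tick calls SetDetination, which issues an AI MoveTo toward the BP_MainPlayer pawn's location plus OffsetToPlayer.
; A successful move sets max walk speed to StopVelocity, with no reset in this graph.
; AnyDamage prints a debug message and enables physics simulation on the mesh.
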(event Custom|SetDetination
  (bind _asbp_main_player (Utilities|Casting|CastToBP_MainPlayer (Game|Player|GetPlayerPawn 0)))
  (AI|AIMoveTo self (+ (.location (Transformation|GetActorTransform _asbp_main_player)) (Variables|Default|GetOffsetToPlayer)) 0 5.0 false
    (:OnSuccess
      (Variables|/Script/Engine.CharacterMovementComponent|SetMaxWalkSpeed (Variables|Character|GetCharacterMovement) (Variables|Default|GetStopVelocity)))))

(event EventBeginPlay)

(event Collision|EventActorBeginOverlap
  (params (OtherActor :type Actor%20Object%20Reference)))

(event EventTick
  (params (DeltaSeconds :type Float%20%28single-precision%29))
  (CallFunction|SetDetination))

(event Game|Damage|EventAnyDamage
  (params (Damage :type Float%20%28single-precision%29) (DamageType :type Damage%20Type%20Object%20Reference) (InstigatedBy :type Controller%20Object%20Reference) (DamageCauser :type Actor%20Object%20Reference))
  (Development|PrintString "recibi daño")
  (Physics|SetSimulatePhysics (Variables|Character|GetMesh) true))

(fn ConstructionScript)